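; Game mode Blueprint that bridges gameplay to the Orchestria network layer for readiness, game start and team scoring.
; A timer started on BeginPlay reports ready after a short delay.
; Update events read network state to set the start delay, started flag and team score, while ReportScore sends scores out.
; ShowScoreScreen refreshes the team score and flips the gameplay HUD's widget switcher to another page.
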(event EventBeginPlay
  (Utilities|Time|SetTimerbyFunctionName 0 "Ready" 3.0))

(event EventTick
  (params (DeltaSeconds :type Float%20%28single-precision%29)))

(event EventReportReady
  (Class|OrchestriaNetworkFunctions|OrchestriaNetworkReportReady))

(event EventUpdateStartedState
  (bind _returnvalue (Class|OrchestriaNetworkFunctions|OrchestriaNetworkGetGameState))
  (if (== _returnvalue 2)
    (bind _returnvalue_2 (Class|OrchestriaNetworkFunctions|OrchestriaNetworkGetStartDelay))
    (Class|OrchestriaGameMode|SetStartDelay _returnvalue_2)
    (Variables|Default|Set_gameStarted true)))

(event EventUpdateGameState
  (bind _returnvalue (Class|OrchestriaNetworkFunctions|OrchestriaNetworkGetScore))
  (Variables|Default|Set_teamScore _returnvalue))

(event EventReportScore
  (params (scoreVal :type Integer))
  (Class|OrchestriaNetworkFunctions|OrchestriaNetworkReportScore scoreVal))

(event EventShowScoreScreen
  (bind _returnvalue (Class|OrchestriaNetworkFunctions|OrchestriaNetworkGetScore))
  (Variables|Default|Set_teamScore _returnvalue)
  (bind _asgameplay_hud (Utilities|Casting|CastToGameplayHUD (Variables|Default|Get_currentWidget)))
  (Class|WidgetSwitcher|SetActiveWidgetIndex (Variables|/Game/Blueprints/GameplayHUD.GameplayHUD_C|GetGameplayHUDSwitcher _asgameplay_hud) 1))

(fn ConstructionScript)

(fn Ready
  (Class|OrchestriaNetworkFunctions|OrchestriaNetworkReportReady))