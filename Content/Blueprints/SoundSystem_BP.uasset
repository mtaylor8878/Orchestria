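; Sound system Blueprint that plays pre-recorded orchestral note samples for brass, drum kit, marimba and timpani as 2D sounds.
; PlaySoundfromLibrary sets a volume multiplier from a musical dynamic, then routes a note struct to per-instrument functions that select samples through nested name, octave and length switches.
; PlayLibrarySound_1 offers a flat enum lookup for percussion only.
; Horn samples call PlaySound2D directly, bypassing the PlaySound helper and its volume multiplier.
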(event Custom|PlayLibrarySound_1
  (params (sound :type Byte) (dynamic :type EDynamic%20Enum :default "EFortissimo"))
  (switch Utilities|FlowControl|Switch|SwitchonEDynamic dynamic
    (:EFortissimo
      (Variables|Default|SetVolumeMultiplier 2.0))
    (:EForte
      (Variables|Default|SetVolumeMultiplier 1.5))
    (:EMezzoForte
      (Variables|Default|SetVolumeMultiplier 1.0))
    (:EMezzoPiano
      (Variables|Default|SetVolumeMultiplier 0.5))
    (:EPiano
      (Variables|Default|SetVolumeMultiplier 0.25))
    (:EPianissimo
      (Variables|Default|SetVolumeMultiplier 0.125)))
  (switch Utilities|FlowControl|Switch|Switchon sound
    (:EDrumKitCrash
      (Variables|Default|SetSound%20to%20Play "/Game/Assets/Audio/Drum_Kit/CrashHit.CrashHit"))
    (:EDrumKitKick
      (Variables|Default|SetSound%20to%20Play "/Game/Assets/Audio/Drum_Kit/KickDrum.KickDrum"))
    (:EDrumKitRim
      (Variables|Default|SetSound%20to%20Play "/Game/Assets/Audio/Drum_Kit/RimShot.RimShot"))
    (:EMarimbaA3
      (Variables|Default|SetSound%20to%20Play "/Game/Assets/Audio/Marimba/MarimbaA3.MarimbaA3"))
    (:EMarimbaA4
      (Variables|Default|SetSound%20to%20Play "/Game/Assets/Audio/Marimba/MarimbaA4.MarimbaA4"))
    (:EMarimbaB3
      (Variables|Default|SetSound%20to%20Play "/Game/Assets/Audio/Marimba/MarimbaB3.MarimbaB3"))
    (:EMarimbaB4
      (Variables|Default|SetSound%20to%20Play "/Game/Assets/Audio/Marimba/MarimbaB4.MarimbaB4"))
    (:EMarimbaB5
      (Variables|Default|SetSound%20to%20Play "/Game/Assets/Audio/Marimba/MarimbaB5.MarimbaB5"))
    (:EMarimbaC4
      (Variables|Default|SetSound%20to%20Play "/Game/Assets/Audio/Marimba/MarimbaC4.MarimbaC4"))
    (:EMarimbaC4S
      (Variables|Default|SetSound%20to%20Play "/Game/Assets/Audio/Marimba/MarimbaC4Sharp.MarimbaC4Sharp"))
    (:EMarimbaC5S
      (Variables|Default|SetSound%20to%20Play "/Game/Assets/Audio/Marimba/MarimbaC5Sharp.MarimbaC5Sharp"))
    (:EMarimbaC6S
      (Variables|Default|SetSound%20to%20Play "/Game/Assets/Audio/Marimba/MarimbaC6Sharp.MarimbaC6Sharp"))
    (:EMarimbaD4
      (Variables|Default|SetSound%20to%20Play "/Game/Assets/Audio/Marimba/MarimbaD4.MarimbaD4"))
    (:EMarimbaD6
      (Variables|Default|SetSound%20to%20Play "/Game/Assets/Audio/Marimba/MarimbaD6.MarimbaD6"))
    (:EMarimbaE3
      (Variables|Default|SetSound%20to%20Play "/Game/Assets/Audio/Marimba/MarimbaE3.MarimbaE3"))
    (:EMarimbaE4
      (Variables|Default|SetSound%20to%20Play "/Game/Assets/Audio/Marimba/MarimbaE4.MarimbaE4"))
    (:EMarimbaF3
      (Variables|Default|SetSound%20to%20Play "/Game/Assets/Audio/Marimba/MarimbaF3.MarimbaF3"))
    (:EMarimbaF3S
      (Variables|Default|SetSound%20to%20Play "/Game/Assets/Audio/Marimba/MarimbaF3Sharp.MarimbaF3Sharp"))
    (:EMarimbaF5S
      (Variables|Default|SetSound%20to%20Play "/Game/Assets/Audio/Marimba/MarimbaF5Sharp.MarimbaF5Sharp"))
    (:EMarimbaG3S
      (Variables|Default|SetSound%20to%20Play "/Game/Assets/Audio/Marimba/MarimbaG3Sharp.MarimbaG3Sharp"))
    (:EMarimbaG4
      (Variables|Default|SetSound%20to%20Play "/Game/Assets/Audio/Marimba/MarimbaG4.MarimbaG4"))
    (:EMarimbaG4S
      (Variables|Default|SetSound%20to%20Play "/Game/Assets/Audio/Marimba/MarimbaG4Sharp.MarimbaG4Sharp"))
    (:EMarimbaG5S
      (Variables|Default|SetSound%20to%20Play "/Game/Assets/Audio/Marimba/MarimbaG5Sharp.MarimbaG5Sharp"))
    (:ETimpaniA2
      (Variables|Default|SetSound%20to%20Play "/Game/Assets/Audio/Timpani/TimpaniA2.TimpaniA2"))
    (:ETimpaniC3S
      (Variables|Default|SetSound%20to%20Play "/Game/Assets/Audio/Timpani/TimpaniC3Sharp.TimpaniC3Sharp"))
    (:ETimpaniD2
      (Variables|Default|SetSound%20to%20Play "/Game/Assets/Audio/Timpani/TimpaniD2.TimpaniD2"))
    (:ETimpaniD3
      (Variables|Default|SetSound%20to%20Play "/Game/Assets/Audio/Timpani/TimpaniD3.TimpaniD3"))
    (:ETimpaniE2
      (Variables|Default|SetSound%20to%20Play "/Game/Assets/Audio/Timpani/TimpaniE2.TimpaniE2"))
    (:ETimpaniE3
      (Variables|Default|SetSound%20to%20Play "/Game/Assets/Audio/Timpani/TimpaniE3.TimpaniE3"))
    (:ETimpaniF2
      (Variables|Default|SetSound%20to%20Play "/Game/Assets/Audio/Timpani/TimpaniF2.TimpaniF2"))
    (:ETimpaniF3S
      (Variables|Default|SetSound%20to%20Play "/Game/Assets/Audio/Timpani/TimpaniF3Sharp.TimpaniF3Sharp"))
    (:ETimpaniG2
      (Variables|Default|SetSound%20to%20Play "/Game/Assets/Audio/Timpani/TimpaniG2.TimpaniG2"))
    (:ETimpaniG2S
      (Variables|Default|SetSound%20to%20Play "/Game/Assets/Audio/Timpani/TimpaniA2Flat.TimpaniA2Flat")))
  (Audio|PlaySound2D (Variables|Default|GetSound%20to%20Play) (Variables|Default|GetVolumeMultiplier) 1.0 0.0 0 0))

(event EventBeginPlay)

(event Collision|EventActorBeginOverlap
  (params (OtherActor :type Actor%20Object%20Reference)))

(event EventTick
  (params (DeltaSeconds :type Float%20%28single-precision%29)))

(event EventPlaySoundfromLibrary
  (params (dynamic :type EDynamic%20Enum :default "EFortissimo") (sound :type Sound%20Identifier%20Structure%20%28by%20ref%29))
  (bind (_instrument _name _octave _length) (Utilities|Struct|BreakSoundIdentifier sound))
  (switch Utilities|FlowControl|Switch|SwitchonEDynamic dynamic
    (:EFortissimo
      (Variables|Default|SetVolumeMultiplier 2.0))
    (:EForte
      (Variables|Default|SetVolumeMultiplier 1.5))
    (:EMezzoForte
      (Variables|Default|SetVolumeMultiplier 1.0))
    (:EMezzoPiano
      (Variables|Default|SetVolumeMultiplier 0.5))
    (:EPiano
      (Variables|Default|SetVolumeMultiplier 0.25))
    (:EPianissimo
      (Variables|Default|SetVolumeMultiplier 0.125)))
  (switch Utilities|FlowControl|Switch|SwitchonEInstrument _instrument
    (:ETrumpet
      (CallFunction|PlayTrumpetSound _length _name _length _octave _octave _length _length))
    (:EFHorn
      (CallFunction|PlayHornSound _name _octave _length _length _octave _length _length _length _octave _length))
    (:ETrombone
      (CallFunction|PlayTromboneSound _octave _length _length _length _octave _length _length _octave _length _length _octave _length _length _octave _length _octave _length _length _octave _length _length _octave _length _name))
    (:ETuba
      (CallFunction|PlayTubaSound _octave _length _length _length _octave _length _length _octave _length _length _octave _length _length _octave _length _octave _length _name _octave _length _length))
    (:EDrumKit
      (CallFunction|PlayDrumKitSound _name))
    (:EMarimba
      (CallFunction|PlayMarimbaSound _octave _octave _octave _octave _octave _octave _octave _name))
    (:ETimpani
      (CallFunction|PlayTimpaniSound _name _octave _octave))))

(fn ConstructionScript)

(fn PlaySound
  (params (Sound :type Sound%20Base%20Object%20Reference))
  (Audio|PlaySound2D Sound (Variables|Default|GetVolumeMultiplier) 1.0 0.0 0 0))

(fn PlayTimpaniSound
  (params (Selection :type ENoteName%20Enum :default "ENoteA") (Selection2 :type Integer) (Selection3 :type Integer))
  (switch Utilities|FlowControl|Switch|SwitchonENoteName Selection
    (:ENoteA
      (CallFunction|PlaySound "/Game/Assets/Audio/Timpani/TimpaniA2.TimpaniA2"))
    (:ENoteCS
      (CallFunction|PlaySound "/Game/Assets/Audio/Timpani/TimpaniC3Sharp.TimpaniC3Sharp"))
    (:ENoteD
      (switch int Selection2
        (:2
          (CallFunction|PlaySound "/Game/Assets/Audio/Timpani/TimpaniD2.TimpaniD2"))
        (:3
          (CallFunction|PlaySound "/Game/Assets/Audio/Timpani/TimpaniD3.TimpaniD3"))))
    (:ENoteE
      (switch int Selection3
        (:2
          (CallFunction|PlaySound "/Game/Assets/Audio/Timpani/TimpaniE2.TimpaniE2"))
        (:3
          (CallFunction|PlaySound "/Game/Assets/Audio/Timpani/TimpaniE3.TimpaniE3"))))
    (:ENoteF
      (CallFunction|PlaySound "/Game/Assets/Audio/Timpani/TimpaniF2.TimpaniF2"))
    (:ENoteFS
      (CallFunction|PlaySound "/Game/Assets/Audio/Timpani/TimpaniF3Sharp.TimpaniF3Sharp"))
    (:ENoteG
      (CallFunction|PlaySound "/Game/Assets/Audio/Timpani/TimpaniG2.TimpaniG2"))
    (:ENoteGS
      (CallFunction|PlaySound "/Game/Assets/Audio/Timpani/TimpaniA2Flat.TimpaniA2Flat"))))

(fn PlayMarimbaSound
  (params (Selection :type Integer) (Selection2 :type Integer) (Selection3 :type Integer) (Selection4 :type Integer) (Selection5 :type Integer) (Selection6 :type Integer) (Selection7 :type Integer) (Selection8 :type ENoteName%20Enum :default "ENoteA"))
  (switch Utilities|FlowControl|Switch|SwitchonENoteName Selection8
    (:ENoteA
      (switch int Selection7
        (:3
          (CallFunction|PlaySound "/Game/Assets/Audio/Marimba/MarimbaA3.MarimbaA3"))
        (:4
          (CallFunction|PlaySound "/Game/Assets/Audio/Marimba/MarimbaA4.MarimbaA4"))))
    (:ENoteB
      (switch int Selection
        (:3
          (CallFunction|PlaySound "/Game/Assets/Audio/Marimba/MarimbaB3.MarimbaB3"))
        (:4
          (CallFunction|PlaySound "/Game/Assets/Audio/Marimba/MarimbaB4.MarimbaB4"))
        (:5
          (CallFunction|PlaySound "/Game/Assets/Audio/Marimba/MarimbaB5.MarimbaB5"))))
    (:ENoteC
      (CallFunction|PlaySound "/Game/Assets/Audio/Marimba/MarimbaC4.MarimbaC4"))
    (:ENoteCS
      (switch int Selection2
        (:4
          (CallFunction|PlaySound "/Game/Assets/Audio/Marimba/MarimbaC4Sharp.MarimbaC4Sharp"))
        (:5
          (CallFunction|PlaySound "/Game/Assets/Audio/Marimba/MarimbaC5Sharp.MarimbaC5Sharp"))
        (:6
          (CallFunction|PlaySound "/Game/Assets/Audio/Marimba/MarimbaC6Sharp.MarimbaC6Sharp"))))
    (:ENoteD
      (switch int Selection3
        (:4
          (CallFunction|PlaySound "/Game/Assets/Audio/Marimba/MarimbaD4.MarimbaD4"))
        (:6
          (CallFunction|PlaySound "/Game/Assets/Audio/Marimba/MarimbaD6.MarimbaD6"))))
    (:ENoteE
      (switch int Selection4
        (:3
          (CallFunction|PlaySound "/Game/Assets/Audio/Marimba/MarimbaE3.MarimbaE3"))
        (:4
          (CallFunction|PlaySound "/Game/Assets/Audio/Marimba/MarimbaE4.MarimbaE4"))))
    (:ENoteF
      (CallFunction|PlaySound "/Game/Assets/Audio/Marimba/MarimbaF3.MarimbaF3"))
    (:ENoteFS
      (switch int Selection5
        (:3
          (CallFunction|PlaySound "/Game/Assets/Audio/Marimba/MarimbaF3Sharp.MarimbaF3Sharp"))
        (:5
          (CallFunction|PlaySound "/Game/Assets/Audio/Marimba/MarimbaF5Sharp.MarimbaF5Sharp"))))
    (:ENoteG
      (CallFunction|PlaySound "/Game/Assets/Audio/Marimba/MarimbaG4.MarimbaG4"))
    (:ENoteGS
      (switch int Selection6
        (:3
          (CallFunction|PlaySound "/Game/Assets/Audio/Marimba/MarimbaG3Sharp.MarimbaG3Sharp"))
        (:4
          (CallFunction|PlaySound "/Game/Assets/Audio/Marimba/MarimbaG4Sharp.MarimbaG4Sharp"))
        (:5
          (CallFunction|PlaySound "/Game/Assets/Audio/Marimba/MarimbaG5Sharp.MarimbaG5Sharp"))))))

(fn PlayDrumKitSound
  (params (Selection :type ENoteName%20Enum :default "ENoteA"))
  (switch Utilities|FlowControl|Switch|SwitchonENoteName Selection
    (:ERimShot
      (CallFunction|PlaySound "/Game/Assets/Audio/Drum_Kit/RimShot.RimShot"))
    (:EKickDrum
      (CallFunction|PlaySound "/Game/Assets/Audio/Drum_Kit/KickDrum.KickDrum"))
    (:ECrashCymbal
      (CallFunction|PlaySound "/Game/Assets/Audio/Drum_Kit/CrashHit.CrashHit"))))

(fn PlayTubaSound
  (params (Selection :type Integer) (Selection2 :type ENoteLength%20Enum :default "EDoubleWhole") (Selection3 :type ENoteLength%20Enum :default "EDoubleWhole") (Selection4 :type ENoteLength%20Enum :default "EDoubleWhole") (Selection5 :type Integer) (Selection6 :type ENoteLength%20Enum :default "EDoubleWhole") (Selection7 :type ENoteLength%20Enum :default "EDoubleWhole") (Selection8 :type Integer) (Selection9 :type ENoteLength%20Enum :default "EDoubleWhole") (Selection10 :type ENoteLength%20Enum :default "EDoubleWhole") (Selection11 :type Integer) (Selection12 :type ENoteLength%20Enum :default "EDoubleWhole") (Selection13 :type ENoteLength%20Enum :default "EDoubleWhole") (Selection14 :type Integer) (Selection15 :type ENoteLength%20Enum :default "EDoubleWhole") (Selection16 :type Integer) (Selection17 :type ENoteLength%20Enum :default "EDoubleWhole") (Selection18 :type ENoteName%20Enum :default "ENoteA") (Selection19 :type Integer) (Selection20 :type ENoteLength%20Enum :default "EDoubleWhole") (Selection21 :type ENoteLength%20Enum :default "EDoubleWhole"))
  (switch Utilities|FlowControl|Switch|SwitchonENoteName Selection18
    (:ENoteA
      (switch int Selection
        (:1
          (switch Utilities|FlowControl|Switch|SwitchonENoteLength Selection2
            (:EDoubleWhole
              (CallFunction|PlaySound "/Game/Assets/Audio/Tuba/TubaA1DoubleWhole.TubaA1DoubleWhole"))
            (:EWhole
              (CallFunction|PlaySound "/Game/Assets/Audio/Tuba/TubaA1Whole.TubaA1Whole"))
            (:EQuarter
              (CallFunction|PlaySound "/Game/Assets/Audio/Tuba/TubaA1Quarter.TubaA1Quarter"))))
        (:2
          (switch Utilities|FlowControl|Switch|SwitchonENoteLength Selection3
            (:EDoubleWhole
              (CallFunction|PlaySound "/Game/Assets/Audio/Tuba/TubaA2DoubleWhole.TubaA2DoubleWhole"))
            (:EWhole
              (CallFunction|PlaySound "/Game/Assets/Audio/Tuba/TubaA2Whole.TubaA2Whole"))
            (:EQuarter
              (CallFunction|PlaySound "/Game/Assets/Audio/Tuba/TubaA2Quarter.TubaA2Quarter"))
            (:EQuarterStacc
              (CallFunction|PlaySound "/Game/Assets/Audio/Tuba/TubaA2QuarterStacc.TubaA2QuarterStacc"))))
        (:3
          (CallFunction|PlaySound "/Game/Assets/Audio/Tuba/TubaA3DotQuarter.TubaA3DotQuarter"))))
    (:ENoteAS
      (CallFunction|PlaySound "/Game/Assets/Audio/Tuba/TubaA1SWhole.TubaA1SWhole"))
    (:ENoteB
      (switch Utilities|FlowControl|Switch|SwitchonENoteLength Selection4
        (:EWhole
          (CallFunction|PlaySound "/Game/Assets/Audio/Tuba/TubaB2Whole.TubaB2Whole"))
        (:EQuarter
          (CallFunction|PlaySound "/Game/Assets/Audio/Tuba/TubaB2Quarter.TubaB2Quarter"))))
    (:ENoteC
      (CallFunction|PlaySound "/Game/Assets/Audio/Tuba/TubaC2Whole.TubaC2Whole"))
    (:ENoteCS
      (switch int Selection5
        (:2
          (switch Utilities|FlowControl|Switch|SwitchonENoteLength Selection6
            (:EWhole
              (CallFunction|PlaySound "/Game/Assets/Audio/Tuba/TubaC2SWhole.TubaC2SWhole"))
            (:EHalf
              (CallFunction|PlaySound "/Game/Assets/Audio/Tuba/TubaC2SHalf.TubaC2SHalf"))
            (:EQuarter
              (CallFunction|PlaySound "/Game/Assets/Audio/Tuba/TubaC2SQuarter.TubaC2SQuarter"))
            (:EQuarterStacc
              (CallFunction|PlaySound "/Game/Assets/Audio/Tuba/TubaC2SQuarterStacc.TubaC2SQuarterStacc"))))
        (:3
          (switch Utilities|FlowControl|Switch|SwitchonENoteLength Selection7
            (:EWhole
              (CallFunction|PlaySound "/Game/Assets/Audio/Tuba/TubaC3SWhole.TubaC3SWhole"))
            (:EHalf
              (CallFunction|PlaySound "/Game/Assets/Audio/Tuba/TubaC3SHalf.TubaC3SHalf"))
            (:EDotQuarter
              (CallFunction|PlaySound "/Game/Assets/Audio/Tuba/TubaC3SDotQuarter.TubaC3SDotQuarter"))
            (:EQuarter
              (CallFunction|PlaySound "/Game/Assets/Audio/Tuba/TubaC3SQuarter.TubaC3SQuarter"))))))
    (:ENoteD
      (switch int Selection8
        (:2
          (switch Utilities|FlowControl|Switch|SwitchonENoteLength Selection9
            (:EDoubleWhole
              (CallFunction|PlaySound "/Game/Assets/Audio/Tuba/TubaD2DoubleWhole.TubaD2DoubleWhole"))
            (:EWhole
              (CallFunction|PlaySound "/Game/Assets/Audio/Tuba/TubaD2Whole.TubaD2Whole"))
            (:EHalf
              (CallFunction|PlaySound "/Game/Assets/Audio/Tuba/TubaD2Half.TubaD2Half"))
            (:EQuarter
              (CallFunction|PlaySound "/Game/Assets/Audio/Tuba/TubaD2Quarter.TubaD2Quarter"))
            (:EQuarterStacc
              (CallFunction|PlaySound "/Game/Assets/Audio/Tuba/TubaD2QuarterStacc.TubaD2QuarterStacc"))))
        (:3
          (switch Utilities|FlowControl|Switch|SwitchonENoteLength Selection10
            (:EWhole
              (CallFunction|PlaySound "/Game/Assets/Audio/Tuba/TubaD3Whole.TubaD3Whole"))
            (:EQuarter
              (CallFunction|PlaySound "/Game/Assets/Audio/Tuba/TubaD3Quarter.TubaD3Quarter"))
            (:EEighth
              (CallFunction|PlaySound "/Game/Assets/Audio/Tuba/TubaD3Eighth.TubaD3Eighth"))))))
    (:ENoteE
      (switch int Selection11
        (:2
          (switch Utilities|FlowControl|Switch|SwitchonENoteLength Selection12
            (:EDoubleWhole
              (CallFunction|PlaySound "/Game/Assets/Audio/Tuba/TubaE2DoubleWhole.TubaE2DoubleWhole"))
            (:EWhole
              (CallFunction|PlaySound "/Game/Assets/Audio/Tuba/TubaE2Whole.TubaE2Whole"))
            (:EHalf
              (CallFunction|PlaySound "/Game/Assets/Audio/Tuba/TubaE2Half.TubaE2Half"))
            (:EQuarter
              (CallFunction|PlaySound "/Game/Assets/Audio/Tuba/TubaE2Quarter.TubaE2Quarter"))
            (:EQuarterStacc
              (CallFunction|PlaySound "/Game/Assets/Audio/Tuba/TubaE2QuarterStacc.TubaE2QuarterStacc"))))
        (:3
          (switch Utilities|FlowControl|Switch|SwitchonENoteLength Selection20
            (:EHalf
              (CallFunction|PlaySound "/Game/Assets/Audio/Tuba/TubaE3Half.TubaE3Half"))
            (:EDotQuarter
              (CallFunction|PlaySound "/Game/Assets/Audio/Tuba/TubaE3DotQuarter.TubaE3DotQuarter"))
            (:EEighth
              (CallFunction|PlaySound "/Game/Assets/Audio/Tuba/TubaE3Eighth.TubaE3Eighth"))))))
    (:ENoteF
      (switch Utilities|FlowControl|Switch|SwitchonENoteLength Selection21
        (:EDoubleWhole
          (CallFunction|PlaySound "/Game/Assets/Audio/Tuba/TubaF2DoubleWhole.TubaF2DoubleWhole"))
        (:EWhole
          (CallFunction|PlaySound "/Game/Assets/Audio/Tuba/TubaF2Whole.TubaF2Whole"))
        (:EQuarterStacc
          (CallFunction|PlaySound "/Game/Assets/Audio/Tuba/TubaF2QuarterStacc.TubaF2QuarterStacc"))))
    (:ENoteFS
      (switch int Selection19
        (:2
          (switch Utilities|FlowControl|Switch|SwitchonENoteLength Selection13
            (:EDoubleWhole
              (CallFunction|PlaySound "/Game/Assets/Audio/Tuba/TubaF2SDoubleWhole.TubaF2SDoubleWhole"))
            (:EDotQuarter
              (CallFunction|PlaySound "/Game/Assets/Audio/Tuba/TubaF2SDotQuarter.TubaF2SDotQuarter"))
            (:EQuarter
              (CallFunction|PlaySound "/Game/Assets/Audio/Tuba/TubaF2SQuarter.TubaF2SQuarter"))
            (:EQuarterStacc
              (CallFunction|PlaySound "/Game/Assets/Audio/Tuba/TubaF2SQuarterStacc.TubaF2SQuarterStacc"))))
        (:3
          (CallFunction|PlaySound "/Game/Assets/Audio/Tuba/TubaF3SEighth.TubaF3SEighth"))))
    (:ENoteG
      (switch int Selection14
        (:1
          (CallFunction|PlaySound "/Game/Assets/Audio/Tuba/TubaG1Half.TubaG1Half"))
        (:2
          (switch Utilities|FlowControl|Switch|SwitchonENoteLength Selection15
            (:EDoubleWhole
              (CallFunction|PlaySound "/Game/Assets/Audio/Tuba/TubaG2DoubleWhole.TubaG2DoubleWhole"))
            (:EWhole
              (CallFunction|PlaySound "/Game/Assets/Audio/Tuba/TubaG2Whole.TubaG2Whole"))
            (:EQuarterStacc
              (CallFunction|PlaySound "/Game/Assets/Audio/Tuba/TubaG2QuarterStacc.TubaG2QuarterStacc"))))))
    (:ENoteGS
      (switch int Selection16
        (:1
          (CallFunction|PlaySound "/Game/Assets/Audio/Tuba/TubaG1SWhole.TubaG1SWhole"))
        (:2
          (switch Utilities|FlowControl|Switch|SwitchonENoteLength Selection17
            (:EWhole
              (CallFunction|PlaySound "/Game/Assets/Audio/Tuba/TubaG2SWhole.TubaG2SWhole"))
            (:EHalf
              (CallFunction|PlaySound "/Game/Assets/Audio/Tuba/TubaG2SHalf.TubaG2SHalf"))
            (:EQuarter
              (CallFunction|PlaySound "/Game/Assets/Audio/Tuba/TubaG2SQuarter.TubaG2SQuarter"))))
        (:3
          (CallFunction|PlaySound "/Game/Assets/Audio/Tuba/TubaG3SDotQuarter.TubaG3SDotQuarter"))))))

(fn PlayTromboneSound
  (params (Selection :type Integer) (Selection2 :type ENoteLength%20Enum :default "EDoubleWhole") (Selection3 :type ENoteLength%20Enum :default "EDoubleWhole") (Selection4 :type ENoteLength%20Enum :default "EDoubleWhole") (Selection5 :type Integer) (Selection6 :type ENoteLength%20Enum :default "EDoubleWhole") (Selection7 :type ENoteLength%20Enum :default "EDoubleWhole") (Selection8 :type Integer) (Selection9 :type ENoteLength%20Enum :default "EDoubleWhole") (Selection10 :type ENoteLength%20Enum :default "EDoubleWhole") (Selection11 :type Integer) (Selection12 :type ENoteLength%20Enum :default "EDoubleWhole") (Selection13 :type ENoteLength%20Enum :default "EDoubleWhole") (Selection14 :type Integer) (Selection15 :type ENoteLength%20Enum :default "EDoubleWhole") (Selection16 :type Integer) (Selection17 :type ENoteLength%20Enum :default "EDoubleWhole") (Selection18 :type ENoteLength%20Enum :default "EDoubleWhole") (Selection19 :type Integer) (Selection20 :type ENoteLength%20Enum :default "EDoubleWhole") (Selection21 :type ENoteLength%20Enum :default "EDoubleWhole") (Selection22 :type Integer) (Selection23 :type ENoteLength%20Enum :default "EDoubleWhole") (Selection24 :type ENoteName%20Enum :default "ENoteA"))
  (switch Utilities|FlowControl|Switch|SwitchonENoteName Selection24
    (:ENoteA
      (switch int Selection
        (:2
          (switch Utilities|FlowControl|Switch|SwitchonENoteLength Selection2
            (:EWhole
              (CallFunction|PlaySound "/Game/Assets/Audio/Trombone/TromboneA2Whole.TromboneA2Whole"))
            (:EDotHalf
              (CallFunction|PlaySound "/Game/Assets/Audio/Trombone/TromboneA2DotHalf.TromboneA2DotHalf"))
            (:EQuarterStacc
              (CallFunction|PlaySound "/Game/Assets/Audio/Trombone/TromboneA2QuarterStacc.TromboneA2QuarterStacc"))
            (:ESixteenth
              (CallFunction|PlaySound "/Game/Assets/Audio/Trombone/TromboneA2Sixteenth.TromboneA2Sixteenth"))))
        (:3
          (switch Utilities|FlowControl|Switch|SwitchonENoteLength Selection3
            (:EWhole
              (CallFunction|PlaySound "/Game/Assets/Audio/Trombone/TromboneA3Whole.TromboneA3Whole"))
            (:EHalf
              (CallFunction|PlaySound "/Game/Assets/Audio/Trombone/TromboneA3Half.TromboneA3Half"))
            (:EEighth
              (CallFunction|PlaySound "/Game/Assets/Audio/Trombone/TromboneA3Eighth.TromboneA3Eighth"))
            (:EEighthStacc
              (CallFunction|PlaySound "/Game/Assets/Audio/Trombone/TromboneA3EighthStacc.TromboneA3EighthStacc"))))))
    (:ENoteAS
      (CallFunction|PlaySound "/Game/Assets/Audio/Trombone/TromboneA2SWhole.TromboneA2SWhole"))
    (:ENoteB
      (switch Utilities|FlowControl|Switch|SwitchonENoteLength Selection4
        (:EWhole
          (CallFunction|PlaySound "/Game/Assets/Audio/Trombone/TromboneB3Whole.TromboneB3Whole"))
        (:EDotHalf
          (CallFunction|PlaySound "/Game/Assets/Audio/Trombone/TromboneB3DotHalf.TromboneB3DotHalf"))
        (:EHalf
          (CallFunction|PlaySound "/Game/Assets/Audio/Trombone/TromboneB3Half.TromboneB3Half"))
        (:EQuarter
          (CallFunction|PlaySound "/Game/Assets/Audio/Trombone/TromboneB3Quarter.TromboneB3Quarter"))
        (:EEighth
          (CallFunction|PlaySound "/Game/Assets/Audio/Trombone/TromboneB3Eighth.TromboneB3Eighth"))))
    (:ENoteC
      (switch int Selection5
        (:3
          (switch Utilities|FlowControl|Switch|SwitchonENoteLength Selection6
            (:EWhole
              (CallFunction|PlaySound "/Game/Assets/Audio/Trombone/TromboneC3Whole.TromboneC3Whole"))
            (:EDotHalf
              (CallFunction|PlaySound "/Game/Assets/Audio/Trombone/TromboneC3DotHalf.TromboneC3DotHalf"))))
        (:4
          (switch Utilities|FlowControl|Switch|SwitchonENoteLength Selection7
            (:EHalf
              (CallFunction|PlaySound "/Game/Assets/Audio/Trombone/TromboneC4Half.TromboneC4Half"))
            (:EQuarter
              (CallFunction|PlaySound "/Game/Assets/Audio/Trombone/TromboneC4Quarter.TromboneC4Quarter"))))))
    (:ENoteCS
      (switch int Selection8
        (:3
          (switch Utilities|FlowControl|Switch|SwitchonENoteLength Selection9
            (:EWhole
              (CallFunction|PlaySound "/Game/Assets/Audio/Trombone/TromboneC3SWhole.TromboneC3SWhole"))
            (:EQuarter
              (CallFunction|PlaySound "/Game/Assets/Audio/Trombone/TromboneC3SQuarter.TromboneC3SQuarter"))))
        (:4
          (switch Utilities|FlowControl|Switch|SwitchonENoteLength Selection10
            (:EWhole
              (CallFunction|PlaySound "/Game/Assets/Audio/Trombone/TromboneC4SEighth.TromboneC4SEighth"))
            (:EHalf
              (CallFunction|PlaySound "/Game/Assets/Audio/Trombone/TromboneC4SHalf.TromboneC4SHalf"))
            (:EDotQuarter
              (CallFunction|PlaySound "/Game/Assets/Audio/Trombone/TromboneC4SDotQuarter.TromboneC4SDotQuarter"))
            (:EEighth
              (CallFunction|PlaySound "/Game/Assets/Audio/Trombone/TromboneC4SEighth.TromboneC4SEighth"))))))
    (:ENoteD
      (switch int Selection11
        (:3
          (switch Utilities|FlowControl|Switch|SwitchonENoteLength Selection12
            (:EDoubleWhole
              (CallFunction|PlaySound "/Game/Assets/Audio/Trombone/TromboneD3DoubleWhole.TromboneD3DoubleWhole"))
            (:EWhole
              (CallFunction|PlaySound "/Game/Assets/Audio/Trombone/TromboneD3Whole.TromboneD3Whole"))
            (:EHalf
              (CallFunction|PlaySound "/Game/Assets/Audio/Trombone/TromboneD3Half.TromboneD3Half"))
            (:EEighth
              (CallFunction|PlaySound "/Game/Assets/Audio/Trombone/TromboneD3Eighth.TromboneD3Eighth"))))
        (:4
          (switch Utilities|FlowControl|Switch|SwitchonENoteLength Selection13
            (:EHalf
              (CallFunction|PlaySound "/Game/Assets/Audio/Trombone/TromboneD4Half.TromboneD4Half"))
            (:EDotQuarter
              (CallFunction|PlaySound "/Game/Assets/Audio/Trombone/TromboneD4DotQuarter.TromboneD4DotQuarter"))
            (:EQuarter
              (CallFunction|PlaySound "/Game/Assets/Audio/Trombone/TromboneD4Quarter.TromboneD4Quarter"))
            (:EEighth
              (CallFunction|PlaySound "/Game/Assets/Audio/Trombone/TromboneD4Eighth.TromboneD4Eighth"))))))
    (:ENoteE
      (switch int Selection14
        (:2
          (CallFunction|PlaySound "/Game/Assets/Audio/Trombone/TromboneE2QuarterStacc.TromboneE2QuarterStacc"))
        (:3
          (switch Utilities|FlowControl|Switch|SwitchonENoteLength Selection15
            (:EWhole
              (CallFunction|PlaySound "/Game/Assets/Audio/Trombone/TromboneE3Whole.TromboneE3Whole"))
            (:EHalf
              (CallFunction|PlaySound "/Game/Assets/Audio/Trombone/TromboneE3Half.TromboneE3Half"))))
        (:4
          (CallFunction|PlaySound "/Game/Assets/Audio/Trombone/TromboneE4Eighth.TromboneE4Eighth"))))
    (:ENoteF
      (switch int Selection16
        (:2
          (CallFunction|PlaySound "/Game/Assets/Audio/Trombone/TromboneF2QuarterStacc.TromboneF2QuarterStacc"))
        (:3
          (switch Utilities|FlowControl|Switch|SwitchonENoteLength Selection17
            (:EWhole
              (CallFunction|PlaySound "/Game/Assets/Audio/Trombone/TromboneF3Whole.TromboneF3Whole"))
            (:EHalf
              (CallFunction|PlaySound "/Game/Assets/Audio/Trombone/TromboneF3Half.TromboneF3Half"))))))
    (:ENoteFS
      (switch Utilities|FlowControl|Switch|SwitchonENoteLength Selection18
        (:EDoubleWhole
          (CallFunction|PlaySound "/Game/Assets/Audio/Trombone/TromboneF3SDoubleWhole.TromboneF3SDoubleWhole"))
        (:EHalf
          (CallFunction|PlaySound "/Game/Assets/Audio/Trombone/TromboneF3SHalf.TromboneF3SHalf"))
        (:EQuarter
          (CallFunction|PlaySound "/Game/Assets/Audio/Trombone/TromboneF3SQuarter.TromboneF3SQuarter"))
        (:EEighth
          (CallFunction|PlaySound "/Game/Assets/Audio/Trombone/TromboneF3SEighth.TromboneF3SEighth"))))
    (:ENoteG
      (switch int Selection19
        (:2
          (switch Utilities|FlowControl|Switch|SwitchonENoteLength Selection20
            (:EHalf
              (CallFunction|PlaySound "/Game/Assets/Audio/Trombone/TromboneG2Half.TromboneG2Half"))
            (:EQuarterStacc
              (CallFunction|PlaySound "/Game/Assets/Audio/Trombone/TromboneG2QuarterStacc.TromboneG2QuarterStacc"))))
        (:3
          (switch Utilities|FlowControl|Switch|SwitchonENoteLength Selection21
            (:EWhole
              (CallFunction|PlaySound "/Game/Assets/Audio/Trombone/TromboneG3Whole.TromboneG3Whole"))
            (:EEighth
              (CallFunction|PlaySound "/Game/Assets/Audio/Trombone/TromboneG3Eighth.TromboneG3Eighth"))))))
    (:ENoteGS
      (switch int Selection22
        (:2
          (CallFunction|PlaySound "/Game/Assets/Audio/Trombone/TromboneG2SWhole.TromboneG2SWhole"))
        (:3
          (switch Utilities|FlowControl|Switch|SwitchonENoteLength Selection23
            (:EDoubleWhole
              (CallFunction|PlaySound "/Game/Assets/Audio/Trombone/TromboneG3SDoubleWhole.TromboneG3SDoubleWhole"))
            (:EWhole
              (CallFunction|PlaySound "/Game/Assets/Audio/Trombone/TromboneG3SWhole.TromboneG3SWhole"))
            (:EDotHalf
              (CallFunction|PlaySound "/Game/Assets/Audio/Trombone/TromboneG3SDotHalf.TromboneG3SDotHalf"))
            (:EHalf
              (CallFunction|PlaySound "/Game/Assets/Audio/Trombone/TromboneG3SHalf.TromboneG3SHalf"))
            (:EEighth
              (CallFunction|PlaySound "/Game/Assets/Audio/Trombone/TromboneG3SEighth.TromboneG3SEighth"))))))))

(fn PlayHornSound
  (params (Selection :type ENoteName%20Enum :default "ENoteA") (Selection2 :type Integer) (Selection3 :type ENoteLength%20Enum :default "EDoubleWhole") (Selection4 :type ENoteLength%20Enum :default "EDoubleWhole") (Selection5 :type Integer) (Selection6 :type ENoteLength%20Enum :default "EDoubleWhole") (Selection7 :type ENoteLength%20Enum :default "EDoubleWhole") (Selection8 :type ENoteLength%20Enum :default "EDoubleWhole") (Selection9 :type Integer) (Selection10 :type ENoteLength%20Enum :default "EDoubleWhole"))
  (switch Utilities|FlowControl|Switch|SwitchonENoteName Selection
    (:ENoteA
      (switch int Selection2
        (:3
          (switch Utilities|FlowControl|Switch|SwitchonENoteLength Selection3
            (:EWhole
              (Audio|PlaySound2D "/Game/Assets/Audio/Horn/HornA3Whole.HornA3Whole" 1.0 1.0 0.0 0 0))
            (:EDotHalf
              (Audio|PlaySound2D "/Game/Assets/Audio/Horn/HornA3DotHalf.HornA3DotHalf" 1.0 1.0 0.0 0 0))))
        (:4
          (Audio|PlaySound2D "/Game/Assets/Audio/Horn/HornA4Quarter.HornA4Quarter" 1.0 1.0 0.0 0 0))))
    (:ENoteB
      (switch Utilities|FlowControl|Switch|SwitchonENoteLength Selection4
        (:EDotHalf
          (Audio|PlaySound2D "/Game/Assets/Audio/Horn/HornB3DotHalf.HornB3DotHalf" 1.0 1.0 0.0 0 0))
        (:EQuarter
          (Audio|PlaySound2D "/Game/Assets/Audio/Horn/HornB3Quarter.HornB3Quarter" 1.0 1.0 0.0 0 0))))
    (:ENoteCS
      (switch int Selection5
        (:3
          (Audio|PlaySound2D "/Game/Assets/Audio/Horn/HornC3SHalf.HornC3SHalf" 1.0 1.0 0.0 0 0))
        (:4
          (switch Utilities|FlowControl|Switch|SwitchonENoteLength Selection6
            (:EDoubleWhole
              (Audio|PlaySound2D "/Game/Assets/Audio/Horn/HornC4SDoubleWhole.HornC4SDoubleWhole" 1.0 1.0 0.0 0 0))
            (:EEighth
              (Audio|PlaySound2D "/Game/Assets/Audio/Horn/HornC4SEighth.HornC4SEighth" 1.0 1.0 0.0 0 0))))))
    (:ENoteD
      (switch Utilities|FlowControl|Switch|SwitchonENoteLength Selection7
        (:EHalf
          (Audio|PlaySound2D "/Game/Assets/Audio/Horn/HornD3Half.HornD3Half" 1.0 1.0 0.0 0 0))
        (:EEighth
          (Audio|PlaySound2D "/Game/Assets/Audio/Horn/HornD3Eighth.HornD3Eighth" 1.0 1.0 0.0 0 0))))
    (:ENoteE
      (Audio|PlaySound2D "/Game/Assets/Audio/Horn/HornE4Eighth.HornE4Eighth" 1.0 1.0 0.0 0 0))
    (:ENoteF
      (Audio|PlaySound2D "/Game/Assets/Audio/Horn/HornF4Half.HornF4Half" 1.0 1.0 0.0 0 0))
    (:ENoteFS
      (switch Utilities|FlowControl|Switch|SwitchonENoteLength Selection8
        (:EDotHalf
          (Audio|PlaySound2D "/Game/Assets/Audio/Horn/HornF4SDotHalf.HornF4SDotHalf" 1.0 1.0 0.0 0 0))
        (:EEighth
          (Audio|PlaySound2D "/Game/Assets/Audio/Horn/HornF4SEighth.HornF4SEighth" 1.0 1.0 0.0 0 0))))
    (:ENoteGS
      (switch int Selection9
        (:3
          (Audio|PlaySound2D "/Game/Assets/Audio/Horn/HornG3SQuarter.HornG3SQuarter" 1.0 1.0 0.0 0 0))
        (:4
          (switch Utilities|FlowControl|Switch|SwitchonENoteLength Selection10
            (:EQuarter
              (Audio|PlaySound2D "/Game/Assets/Audio/Horn/HornG4SQuarter.HornG4SQuarter" 1.0 1.0 0.0 0 0))
            (:EEighth
              (Audio|PlaySound2D "/Game/Assets/Audio/Horn/HornG4SEighth.HornG4SEighth" 1.0 1.0 0.0 0 0))))))))

(fn PlayTrumpetSound
  (params (Selection :type ENoteLength%20Enum :default "EDoubleWhole") (Selection2 :type ENoteName%20Enum :default "ENoteA") (Selection3 :type ENoteLength%20Enum :default "EDoubleWhole") (Selection4 :type Integer) (Selection5 :type Integer) (Selection6 :type ENoteLength%20Enum :default "EDoubleWhole") (Selection7 :type ENoteLength%20Enum :default "EDoubleWhole"))
  (switch Utilities|FlowControl|Switch|SwitchonENoteName Selection2
    (:ENoteA
      (switch Utilities|FlowControl|Switch|SwitchonENoteLength Selection
        (:EWhole
          (CallFunction|PlaySound "/Game/Assets/Audio/Trumpet/TrumpetA4Whole.TrumpetA4Whole"))
        (:EDotHalf
          (CallFunction|PlaySound "/Game/Assets/Audio/Trumpet/TrumpetA4DotHalf.TrumpetA4DotHalf"))
        (:EEighth
          (CallFunction|PlaySound "/Game/Assets/Audio/Trumpet/TrumpetA4Eighth.TrumpetA4Eighth"))))
    (:ENoteB
      (switch Utilities|FlowControl|Switch|SwitchonENoteLength Selection3
        (:EDotHalf
          (CallFunction|PlaySound "/Game/Assets/Audio/Trumpet/TrumpetB4DotHalf.TrumpetB4DotHalf"))
        (:EEighth
          (CallFunction|PlaySound "/Game/Assets/Audio/Trumpet/TrumpetB4Eighth.TrumpetB4Eighth"))))
    (:ENoteCS
      (switch int Selection4
        (:4
          (CallFunction|PlaySound "/Game/Assets/Audio/Trumpet/TrumpetC4SDotHalf.TrumpetC4SDotHalf"))
        (:5
          (CallFunction|PlaySound "/Game/Assets/Audio/Trumpet/TrumpetC5SEighth.TrumpetC5SEighth"))))
    (:ENoteD
      (CallFunction|PlaySound "/Game/Assets/Audio/Trumpet/TrumpetD5Eighth.TrumpetD5Eighth"))
    (:ENoteE
      (switch int Selection5
        (:4
          (CallFunction|PlaySound "/Game/Assets/Audio/Trumpet/TrumpetE4Eighth.TrumpetE4Eighth"))
        (:5
          (CallFunction|PlaySound "/Game/Assets/Audio/Trumpet/TrumpetE5Eighth.TrumpetE5Eighth"))))
    (:ENoteF
      (switch Utilities|FlowControl|Switch|SwitchonENoteLength Selection6
        (:EWhole
          (CallFunction|PlaySound "/Game/Assets/Audio/Trumpet/TrumpetF4Whole.TrumpetF4Whole"))
        (:EEighth
          (CallFunction|PlaySound "/Game/Assets/Audio/Trumpet/TrumpetF4Eighth.TrumpetF4Eighth"))))
    (:ENoteFS
      (CallFunction|PlaySound "/Game/Assets/Audio/Trumpet/TrumpetF4SEighth.TrumpetF4SEighth"))
    (:ENoteGS
      (switch Utilities|FlowControl|Switch|SwitchonENoteLength Selection7
        (:EDotHalf
          (CallFunction|PlaySound "/Game/Assets/Audio/Trumpet/TrumpetG4SDotHalf.TrumpetG4SDotHalf"))
        (:EEighth
          (CallFunction|PlaySound "/Game/Assets/Audio/Trumpet/TrumpetG4SEighth.TrumpetG4SEighth"))))))